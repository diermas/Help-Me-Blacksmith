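; Customer Blueprint that generates a randomized weapon request and shows it to the player as dialog.
; On BeginPlay it rolls weight, length, handling and sharpness requirements, each of which can be "None".
; It appends the specified requirements into one sentence, converts it to text, and passes it to a new CustomerDialog_BP widget added to the viewport.
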(event EventBeginPlay
  (switch int (Math|Random|RandomInteger 3)
    (:0
      (Variables|Default|SetReqWeight "Heavy"))
    (:1
      (Variables|Default|SetReqWeight "Light"))
    (:2
      (Variables|Default|SetReqWeight "None")))
  (switch int (Math|Random|RandomInteger 3)
    (:0
      (Variables|Default|SetReqLength "Long"))
    (:1
      (Variables|Default|SetReqLength "Short"))
    (:2
      (Variables|Default|SetReqLength "None")))
  (switch int (Math|Random|RandomInteger 3)
    (:0
      (Variables|Default|SetReqHandling "Fast"))
    (:1
      (Variables|Default|SetReqHandling "Slow"))
    (:2
      (Variables|Default|SetReqHandling "None")))
  (switch int (Math|Random|RandomInteger 3)
    (:0
      (Variables|Default|SetReqSharp "Sharp"))
    (:1
      (Variables|Default|SetReqSharp "Blunt"))
    (:2
      (Variables|Default|SetReqSharp "None")))
  (bind _output_get (Variables|Default|SetDialogString "I need a weapon that is "))
  (if (Utilities|Enum|Equal(Enum) (Variables|Default|GetReqWeight) "None")
    _
    (else
      (Variables|Default|SetDialogString (Utilities|String|Append (Utilities|String|Append _output_get (Variables|Default|GetReqWeight)) " weight, "))))
  (if (Utilities|Enum|Equal(Enum) (Variables|Default|GetReqLength) "None")
    _
    (else
      (Variables|Default|SetDialogString (Utilities|String|Append (Utilities|String|Append (Variables|Default|GetDialogString) (Variables|Default|GetReqLength)) " length, "))))
  (if (Utilities|Enum|Equal(Enum) (Variables|Default|GetReqHandling) "None")
    _
    (else
      (Variables|Default|SetDialogString (Utilities|String|Append (Utilities|String|Append (Variables|Default|GetDialogString) (Variables|Default|GetReqHandling)) " speed, "))))
  (if (Utilities|Enum|Equal(Enum) (Variables|Default|GetReqSharp) "None")
    _
    (else
      (Variables|Default|SetDialogString (Utilities|String|Append (Utilities|String|Append (Variables|Default|GetDialogString) (Variables|Default|GetReqSharp)) "."))))
  (bind _output_get_2 (Variables|Default|SetDialog (Utilities|Text|ToText(String) (Variables|Default|GetDialogString))))
  (bind _returnvalue (UserInterface|CreateWidget "/Game/Blueprints/CustomerDialog_BP.CustomerDialog_BP_C" (Game|GetPlayerController 0)))
  (Variables|/Game/Blueprints/CustomerDialog_BP.CustomerDialog_BP_C|SetDialogText _returnvalue _output_get_2)
  (UserInterface|Viewport|AddtoViewport _returnvalue 0))

(fn ConstructionScript)