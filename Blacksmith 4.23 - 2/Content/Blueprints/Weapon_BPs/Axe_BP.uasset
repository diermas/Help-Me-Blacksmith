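; Axe weapon Blueprint that defines the axe's stats on top of a parent class.
; BeginPlay runs the parent logic, then sets fixed values for Weight, Length, Sharpness, Defense and Handling.
; Overlap and construction only call the parent, and Tick is disabled, so the axe adds no behavior of its own beyond those stats.
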(event EventBeginPlay
  (|CallParentFunction)
  (Variables|Default|SetWeight 1)
  (Variables|Default|SetLength 1)
  (Variables|Default|SetSharpness 0)
  (Variables|Default|SetDefense 2)
  (Variables|Default|SetHandling 3))

(event Collision|EventActorBeginOverlap
  (params (OtherActor :type Actor%20Object%20Reference))
  (|CallParentFunction OtherActor))

(event EventTick
  (params (DeltaSeconds :type Float%20%28single-precision%29))
  (|CallParentFunction DeltaSeconds) ; This node is disabled and will not be called.\nDrag off pins to build functionality.
)

(fn ConstructionScript
  (|CallParentFunction))