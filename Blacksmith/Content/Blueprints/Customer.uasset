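; Customer actor that generates a random weapon order and presents it to the player as dialog.
; On BeginPlay it randomly rolls weight, length, handling and sharpness requirements, each possibly "None", appends the non-None ones into a sentence and shows it in a CustomerDialog_BP widget.
; WeaponDone opens a NextCustomer_BP widget with button and evaluation visible, using placeholder "TEST" text rather than scoring the weapon against the request.
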(event Custom|Weapon%20Done
  (bind _returnvalue (UserInterface|CreateWidget "/Game/Blueprints/NextCustomer_BP.NextCustomer_BP_C"))
  (Variables|/Game/Blueprints/NextCustomer_BP.NextCustomer_BP_C|SetTextVis _returnvalue false)
  (Variables|/Game/Blueprints/NextCustomer_BP.NextCustomer_BP_C|SetButtonVis _returnvalue true)
  (Variables|/Game/Blueprints/NextCustomer_BP.NextCustomer_BP_C|SetEvalVis _returnvalue true)
  (Variables|/Game/Blueprints/NextCustomer_BP.NextCustomer_BP_C|SetCustomer%20Evaluation _returnvalue "TEST")
  (UserInterface|Viewport|AddtoViewport _returnvalue 0))

(event EventBeginPlay
  (switch int (Math|Random|RandomInteger 3)
    (:0
      (Variables|Default|SetReqWeight "heavy"))
    (:1
      (Variables|Default|SetReqWeight "light"))
    (:2
      (Variables|Default|SetReqWeight "None")))
  (switch int (Math|Random|RandomInteger 3)
    (:0
      (Variables|Default|SetReqLength "long"))
    (:1
      (Variables|Default|SetReqLength "short"))
    (:2
      (Variables|Default|SetReqLength "None")))
  (switch int (Math|Random|RandomInteger 3)
    (:0
      (Variables|Default|SetReqHandling "fast"))
    (:1
      (Variables|Default|SetReqHandling "slow"))
    (:2
      (Variables|Default|SetReqHandling "None")))
  (switch int (Math|Random|RandomInteger 3)
    (:0
      (Variables|Default|SetReqSharp "sharp"))
    (:1
      (Variables|Default|SetReqSharp "blunt"))
    (:2
      (Variables|Default|SetReqSharp "None")))
  (bind _output_get (Variables|Default|SetDialogString "I need a weapon that is "))
  (if (Utilities|Enum|Equal(Enum) (Variables|Default|GetReqWeight) "None")
    _
    (else
      (Variables|Default|SetDialogString (Utilities|String|Append (Utilities|String|Append _output_get (Variables|Default|GetReqWeight)) " weight, "))))
  (if (Utilities|Enum|Equal(Enum) (Variables|Default|GetReqLength) "None")
    _
    (else
      (Variables|Default|SetDialogString (Utilities|String|Append (Utilities|String|Append (Variables|Default|GetDialogString) (Variables|Default|GetReqLength)) " length, "))))
  (if (Utilities|Enum|Equal(Enum) (Variables|Default|GetReqHandling) "None")
    _
    (else
      (Variables|Default|SetDialogString (Utilities|String|Append (Utilities|String|Append (Variables|Default|GetDialogString) (Variables|Default|GetReqHandling)) " speed, "))))
  (if (Utilities|Enum|Equal(Enum) (Variables|Default|GetReqSharp) "None")
    _
    (else
      (Variables|Default|SetDialogString (Utilities|String|Append (Utilities|String|Append (Variables|Default|GetDialogString) (Variables|Default|GetReqSharp)) "."))))
  (bind _output_get_2 (Variables|Default|SetDialog (Utilities|Text|ToText(String) (Variables|Default|GetDialogString))))
  (bind _returnvalue (UserInterface|CreateWidget "/Game/Blueprints/CustomerDialog_BP.CustomerDialog_BP_C" (Game|GetPlayerController 0)))
  (Variables|/Game/Blueprints/CustomerDialog_BP.CustomerDialog_BP_C|SetDialogText _returnvalue _output_get_2)
  (UserInterface|Viewport|AddtoViewport _returnvalue 0))

(fn ConstructionScript)