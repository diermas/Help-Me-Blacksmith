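; LevelController_BP is a controller actor for a weapon-crafting customer loop, exposing events to spawn customers, begin crafting and finish a weapon.
; BeginCrafting spawns WeaponBuilder_BP and reveals the Options_BP widgets.
; WeaponDone destroys the first handle, guard and weapon head found by class lookup, then calls WeaponDone on the first Customer.
; An unconnected chain for showing the NextCustomer_BP widget and removing the customer never runs.
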(event Custom|Spawn%20Customer
  (Game|SpawnActorfromClass "/Game/Blueprints/Customer.Customer_C" (Math|Transform|MakeTransform "0, 0, 0" "0, 0, 0" "1,1,1") "AlwaysSpawn" 0 0))

(event Custom|Weapon%20Done
  (bind _outactors (Actor|GetAllActorsOfClass "/Game/Blueprints/Weapon_BPs/Handle_BP.Handle_BP_C"))
  (Actor|DestroyActor (Utilities|Array|Get(acopy) _outactors))
  (bind _outactors_2 (Actor|GetAllActorsOfClass "/Game/Blueprints/Weapon_BPs/Guard_BP.Guard_BP_C"))
  (Actor|DestroyActor (Utilities|Array|Get(acopy) _outactors_2))
  (bind _outactors_3 (Actor|GetAllActorsOfClass "/Game/Blueprints/Weapon_BPs/WeaponHead_BP.WeaponHead_BP_C"))
  (Actor|DestroyActor (Utilities|Array|Get(acopy) _outactors_3))
  (bind _outactors_4 (Actor|GetAllActorsOfClass "/Game/Blueprints/Customer.Customer_C"))
  (Default|WeaponDone (Utilities|Array|Get(acopy) _outactors_4)))

(event Custom|Begin%20Crafting
  (Game|SpawnActorfromClass "/Game/Blueprints/WeaponBuilder_BP.WeaponBuilder_BP_C" (Math|Transform|MakeTransform "0, 0, 0" "0, 0, 0" "1,1,1") "AlwaysSpawn" 0 0)
  (bind _foundwidgets (Widget|GetAllWidgetsOfClass "/Game/Blueprints/Options_BP.Options_BP_C" true))
  (Widget|SetVisibility _foundwidgets "Visible"))

(fn ConstructionScript)