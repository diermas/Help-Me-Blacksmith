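; AxeGuard_BP is a weapon-part Blueprint for an axe guard.
; On BeginPlay it calls the parent, then sets its name and stats for weight, length, sharpness, defense and handling.
; Overlap and construction logic only forward to the parent class, and Tick is disabled, so the asset acts as a data-only variant of its parent.
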(event EventBeginPlay
  (|CallParentFunction)
  (Variables|Default|SetWeight 4)
  (Variables|Default|SetLength 3)
  (Variables|Default|SetSharpness 1)
  (Variables|Default|SetDefense 0)
  (Variables|Default|SetHandling 5)
  (Variables|Default|SetName "Axe Guard"))

(event Collision|EventActorBeginOverlap
  (params (OtherActor :type Actor%20Object%20Reference))
  (|CallParentFunction OtherActor))

(event EventTick
  (params (DeltaSeconds :type Float%20%28single-precision%29))
  (|CallParentFunction DeltaSeconds) ; This node is disabled and will not be called.\nDrag off pins to build functionality.
)

(fn ConstructionScript
  (|CallParentFunction))