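; FinishedWeapon_BP is the assembled weapon actor, built from head, guard and handle parts.
; BuildSet plays a Choir audio event and assigns the chosen classes to the three child actor components.
; It then totals length, weight and handling across the parts, taking sharpness from the head alone.
; Part stats come from world-wide GetActorOfClass lookups rather than from the child actor components.
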(event Custom|Build%20Set
  (Class|FMODBlueprintStatics|PlayEventatLocation "/Game/FMOD/Events/choir.choir" (Transformation|GetActorTransform))
  (ChildActorComponent|SetChildActorClass (Variables|Default|GetWeapon%20Tip) (Variables|Default|GetWeaponClass))
  (ChildActorComponent|SetChildActorClass (Variables|Default|GetGuard) (Variables|Default|GetGuardClass))
  (ChildActorComponent|SetChildActorClass (Variables|Default|GetHandle) (Variables|Default|GetHandleClass))
  (bind _returnvalue (Actor|GetActorOfClass "/Game/Blueprints/Weapon_BPs/WeaponHead_BP.WeaponHead_BP_C"))
  (Variables|Default|SetTotalLength (Variables|/Game/Blueprints/Weapon_BPs/WeaponHead_BP.WeaponHead_BP_C|GetLength _returnvalue))
  (Variables|Default|SetTotalSharp (Variables|/Game/Blueprints/Weapon_BPs/WeaponHead_BP.WeaponHead_BP_C|GetSharpness _returnvalue))
  (Variables|Default|SetTotalWeight (Variables|/Game/Blueprints/Weapon_BPs/WeaponHead_BP.WeaponHead_BP_C|GetWeight _returnvalue))
  (Variables|Default|SetTotalHandling (Variables|/Game/Blueprints/Weapon_BPs/WeaponHead_BP.WeaponHead_BP_C|GetHandling _returnvalue))
  (bind _returnvalue_2 (Actor|GetActorOfClass "/Game/Blueprints/Weapon_BPs/Handle_BP.Handle_BP_C"))
  (Variables|Default|SetTotalLength (+ (Variables|/Game/Blueprints/Weapon_BPs/Handle_BP.Handle_BP_C|GetLength _returnvalue_2) (Variables|Default|GetTotalLength)))
  (Variables|Default|SetTotalWeight (+ (Variables|/Game/Blueprints/Weapon_BPs/Handle_BP.Handle_BP_C|GetWeight _returnvalue_2) (Variables|Default|GetTotalWeight)))
  (Variables|Default|SetTotalHandling (+ (Variables|/Game/Blueprints/Weapon_BPs/Handle_BP.Handle_BP_C|GetHandling _returnvalue_2) (Variables|Default|GetTotalHandling)))
  (bind _returnvalue_3 (Actor|GetActorOfClass "/Game/Blueprints/Weapon_BPs/Guard_BP.Guard_BP_C"))
  (Variables|Default|SetTotalLength (+ (Variables|/Game/Blueprints/Weapon_BPs/Guard_BP.Guard_BP_C|GetLength _returnvalue_3) (Variables|Default|GetTotalLength)))
  (Variables|Default|SetTotalWeight (+ (Variables|/Game/Blueprints/Weapon_BPs/Guard_BP.Guard_BP_C|GetWeight _returnvalue_3) (Variables|Default|GetTotalWeight)))
  (Variables|Default|SetTotalHandling (+ (Variables|/Game/Blueprints/Weapon_BPs/Guard_BP.Guard_BP_C|GetHandling _returnvalue_3) (Variables|Default|GetTotalHandling))))

(fn ConstructionScript)