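; Customer actor that orders a randomly specified weapon and grades the one the player makes.
; On BeginPlay it rolls optional weight, length, handling and sharpness requirements and shows them as a sentence in a CustomerDialog_BP widget.
; WeaponDone compares the first FinishedWeapon_BP's totals to fixed thresholds, scoring equally for each met or unspecified requirement.
; It then shows the score and failed criteria in a NextCustomer_BP widget and destroys itself.
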(event Custom|Weapon%20Done
  (bind _returnvalue (UserInterface|CreateWidget "/Game/Blueprints/NextCustomer_BP.NextCustomer_BP_C"))
  (Variables|/Game/Blueprints/NextCustomer_BP.NextCustomer_BP_C|SetTextVis _returnvalue false)
  (Variables|/Game/Blueprints/NextCustomer_BP.NextCustomer_BP_C|SetButtonVis _returnvalue true)
  (Variables|/Game/Blueprints/NextCustomer_BP.NextCustomer_BP_C|SetEvalVis _returnvalue true)
  (bind _outactors (Actor|GetAllActorsOfClass "/Game/Blueprints/Weapon_BPs/FinishedWeapon_BP.FinishedWeapon_BP_C"))
  (if (Utilities|Enum|Equal(Enum) (Variables|Default|GetReqWeight) "heavy")
    (if (>= (Variables|/Game/Blueprints/Weapon_BPs/FinishedWeapon_BP.FinishedWeapon_BP_C|GetTotalWeight (Utilities|Array|Get(acopy) _outactors)) 11)
      (Variables|Default|SetWeightMet true)
      (Variables|Default|SetScore (+ (Variables|Default|GetScore) 25)))
    (elif (Utilities|Enum|Equal(Enum) (Variables|Default|GetReqWeight) "light")
      (if (>= (Variables|/Game/Blueprints/Weapon_BPs/FinishedWeapon_BP.FinishedWeapon_BP_C|GetTotalWeight (Utilities|Array|Get(acopy) _outactors)) 11)
        _
        (else
          (Variables|Default|SetWeightMet true)
          (Variables|Default|SetScore (+ (Variables|Default|GetScore) 25) :!label _label)))
      (else
        (Variables|Default|SetWeightMet true)
        (goto _label))))
  (if (Utilities|Enum|Equal(Enum) (Variables|Default|GetReqLength) "long")
    (if (>= (Variables|/Game/Blueprints/Weapon_BPs/FinishedWeapon_BP.FinishedWeapon_BP_C|GetTotalLength (Utilities|Array|Get(acopy) _outactors)) 8)
      (Variables|Default|SetLengthMet true)
      (Variables|Default|SetScore (+ (Variables|Default|GetScore) 25)))
    (elif (Utilities|Enum|Equal(Enum) (Variables|Default|GetReqLength) "short")
      (if (>= (Variables|/Game/Blueprints/Weapon_BPs/FinishedWeapon_BP.FinishedWeapon_BP_C|GetTotalLength (Utilities|Array|Get(acopy) _outactors)) 8)
        _
        (else
          (Variables|Default|SetLengthMet true)
          (Variables|Default|SetScore (+ (Variables|Default|GetScore) 25) :!label _label_2)))
      (else
        (Variables|Default|SetLengthMet true)
        (goto _label_2))))
  (if (Utilities|Enum|Equal(Enum) (Variables|Default|GetReqHandling) "fast")
    (if (>= (Variables|/Game/Blueprints/Weapon_BPs/FinishedWeapon_BP.FinishedWeapon_BP_C|GetTotalHandling (Utilities|Array|Get(acopy) _outactors)) 13)
      (Variables|Default|SetHandlingMet true)
      (Variables|Default|SetScore (+ (Variables|Default|GetScore) 25)))
    (elif (Utilities|Enum|Equal(Enum) (Variables|Default|GetReqHandling) "slow")
      (if (>= (Variables|/Game/Blueprints/Weapon_BPs/FinishedWeapon_BP.FinishedWeapon_BP_C|GetTotalHandling (Utilities|Array|Get(acopy) _outactors)) 13)
        _
        (else
          (Variables|Default|SetHandlingMet true)
          (Variables|Default|SetScore (+ (Variables|Default|GetScore) 25) :!label _label_3)))
      (else
        (Variables|Default|SetHandlingMet true)
        (goto _label_3))))
  (if (Utilities|Enum|Equal(Enum) (Variables|Default|GetReqSharp) "sharp")
    (if (== (Variables|/Game/Blueprints/Weapon_BPs/FinishedWeapon_BP.FinishedWeapon_BP_C|GetTotalSharp (Utilities|Array|Get(acopy) _outactors)) 1)
      (Variables|Default|SetSharpMet true)
      (Variables|Default|SetScore (+ (Variables|Default|GetScore) 25)))
    (elif (Utilities|Enum|Equal(Enum) (Variables|Default|GetReqSharp) "blunt")
      (if (== (Variables|/Game/Blueprints/Weapon_BPs/FinishedWeapon_BP.FinishedWeapon_BP_C|GetTotalSharp (Utilities|Array|Get(acopy) _outactors)) 1)
        _
        (else
          (Variables|Default|SetSharpMet true)
          (Variables|Default|SetScore (+ (Variables|Default|GetScore) 25) :!label _label_4)))
      (else
        (Variables|Default|SetSharpMet true)
        (goto _label_4))))
  (Variables|Default|SetDialogString (Utilities|String|Append (Utilities|String|Append "Score: " (Utilities|String|ToString(Integer) (Variables|Default|GetScore))) "."))
  (if (Variables|Default|GetWeightMet)
    _
    (else
      (Variables|Default|SetDialogString (Utilities|String|Append (Variables|Default|GetDialogString) " It was the wrong weight."))))
  (if (Variables|Default|GetLengthMet)
    _
    (else
      (Variables|Default|SetDialogString (Utilities|String|Append (Variables|Default|GetDialogString) " It was the wrong length."))))
  (if (Variables|Default|GetSharpMet)
    _
    (else
      (Variables|Default|SetDialogString (Utilities|String|Append (Variables|Default|GetDialogString) " It was the wrong sharpness."))))
  (if (Variables|Default|GetHandlingMet)
    _
    (else
      (Variables|Default|SetDialogString (Utilities|String|Append (Variables|Default|GetDialogString) " It was the wrong speed."))))
  (Variables|/Game/Blueprints/NextCustomer_BP.NextCustomer_BP_C|SetCustomer%20Evaluation _returnvalue (Utilities|Text|ToText(String) (Variables|Default|GetDialogString)))
  (UserInterface|Viewport|AddtoViewport _returnvalue 0)
  (Actor|DestroyActor))

(event EventBeginPlay
  (switch int (Math|Random|RandomInteger 3)
    (:0
      (Variables|Default|SetReqWeight "heavy"))
    (:1
      (Variables|Default|SetReqWeight "light"))
    (:2
      (Variables|Default|SetReqWeight "None")))
  (switch int (Math|Random|RandomInteger 3)
    (:0
      (Variables|Default|SetReqLength "long"))
    (:1
      (Variables|Default|SetReqLength "short"))
    (:2
      (Variables|Default|SetReqLength "None")))
  (switch int (Math|Random|RandomInteger 3)
    (:0
      (Variables|Default|SetReqHandling "fast"))
    (:1
      (Variables|Default|SetReqHandling "slow"))
    (:2
      (Variables|Default|SetReqHandling "None")))
  (switch int (Math|Random|RandomInteger 3)
    (:0
      (Variables|Default|SetReqSharp "sharp"))
    (:1
      (Variables|Default|SetReqSharp "blunt"))
    (:2
      (Variables|Default|SetReqSharp "None")))
  (bind _output_get (Variables|Default|SetDialogString "I need a weapon that is "))
  (if (Utilities|Enum|Equal(Enum) (Variables|Default|GetReqWeight) "None")
    _
    (else
      (Variables|Default|SetDialogString (Utilities|String|Append (Utilities|String|Append _output_get (Variables|Default|GetReqWeight)) " weight, "))))
  (if (Utilities|Enum|Equal(Enum) (Variables|Default|GetReqLength) "None")
    _
    (else
      (Variables|Default|SetDialogString (Utilities|String|Append (Utilities|String|Append (Variables|Default|GetDialogString) (Variables|Default|GetReqLength)) " length, "))))
  (if (Utilities|Enum|Equal(Enum) (Variables|Default|GetReqHandling) "None")
    _
    (else
      (Variables|Default|SetDialogString (Utilities|String|Append (Utilities|String|Append (Variables|Default|GetDialogString) (Variables|Default|GetReqHandling)) " speed, "))))
  (if (Utilities|Enum|Equal(Enum) (Variables|Default|GetReqSharp) "None")
    _
    (else
      (Variables|Default|SetDialogString (Utilities|String|Append (Utilities|String|Append (Variables|Default|GetDialogString) (Variables|Default|GetReqSharp)) "."))))
  (bind _output_get_2 (Variables|Default|SetDialog (Utilities|Text|ToText(String) (Variables|Default|GetDialogString))))
  (bind _returnvalue (UserInterface|CreateWidget "/Game/Blueprints/CustomerDialog_BP.CustomerDialog_BP_C" (Game|GetPlayerController 0)))
  (Variables|/Game/Blueprints/CustomerDialog_BP.CustomerDialog_BP_C|SetDialogText _returnvalue _output_get_2)
  (UserInterface|Viewport|AddtoViewport _returnvalue 0))

(fn ConstructionScript)