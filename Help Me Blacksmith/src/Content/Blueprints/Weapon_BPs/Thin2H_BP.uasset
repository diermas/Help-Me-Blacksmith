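; Thin2H_BP is a weapon part Blueprint for the "Thin 2H Pommel".
; On BeginPlay it calls the parent, then sets its display name and its Weight, Length, Sharpness, Defense and Handling stats.
; It adds no other active logic: overlap and tick are disabled, and the construction script only calls the parent.
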(event EventBeginPlay
  (|CallParentFunction)
  (Variables|Default|SetWeight 2)
  (Variables|Default|SetLength 2)
  (Variables|Default|SetSharpness 0)
  (Variables|Default|SetDefense 0)
  (Variables|Default|SetHandling 3)
  (Variables|Default|SetName "Thin 2H Pommel"))

(event Collision|EventActorBeginOverlap
  (params (OtherActor :type Actor%20Object%20Reference))
  (|CallParentFunction OtherActor) ; This node is disabled and will not be called.\nDrag off pins to build functionality.
)

(event EventTick
  (params (DeltaSeconds :type Float%20%28single-precision%29))
  (|CallParentFunction DeltaSeconds) ; This node is disabled and will not be called.\nDrag off pins to build functionality.
)

(fn ConstructionScript
  (|CallParentFunction))